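; Player-controlled ship pawn that turns, looks around and fights with cannons through its ArtilleryComponent.
; Input axes drive camera look, ship yaw and cannon pitch, with the ship rotated directly by the raw axis value.
; Holding the aim axis sets the aiming state and draws the trajectory, and Fire shoots only while aiming.
; Three actions switch ammo between round shot, buckshot and knippels, printing the selected type.
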(event EventBeginPlay)

(event Collision|EventActorBeginOverlap
  (params (OtherActor :type Actor%20Object%20Reference)))

(event EventTick
  (params (DeltaSeconds :type Float%20%28single-precision%29)))

(event Input|ActionEvents|InputActionFire
  (params (Key :type Key%20Structure :default "None"))
  (:Pressed
    (if (Variables|/Game/Blueprints/Components/ArtilleryComponent.ArtilleryComponent_C|GetIsAiming (Variables|Default|GetArtilleryComponent))
      (Default|Shoot (Variables|Default|GetArtilleryComponent)))))

(event Input|ActionEvents|InputActionSetBuckshot
  (params (Key :type Key%20Structure :default "None"))
  (:Pressed
    (bind _output_get (Variables|/Game/Blueprints/Components/ArtilleryComponent.ArtilleryComponent_C|SetBallType (Variables|Default|GetArtilleryComponent) "NewEnumerator1"))
    (Development|PrintString (Utilities|String|EnumtoString _output_get))))

(event Input|ActionEvents|InputActionSetRoundShot
  (params (Key :type Key%20Structure :default "None"))
  (:Pressed
    (bind _output_get (Variables|/Game/Blueprints/Components/ArtilleryComponent.ArtilleryComponent_C|SetBallType (Variables|Default|GetArtilleryComponent) "NewEnumerator0"))
    (Development|PrintString (Utilities|String|EnumtoString _output_get))))

(event Input|ActionEvents|InputActionSetKnippels
  (params (Key :type Key%20Structure :default "None"))
  (:Pressed
    (bind _output_get (Variables|/Game/Blueprints/Components/ArtilleryComponent.ArtilleryComponent_C|SetBallType (Variables|Default|GetArtilleryComponent) "NewEnumerator2"))
    (Development|PrintString (Utilities|String|EnumtoString _output_get))))

(event Input|AxisEvents|InputAxisLookUp
  (params (AxisValue :type Float%20%28single-precision%29))
  (Pawn|Input|AddControllerPitchInput AxisValue))

(event Input|AxisEvents|InputAxisTurn
  (params (AxisValue :type Float%20%28single-precision%29))
  (Pawn|Input|AddControllerYawInput AxisValue))

(event Input|AxisEvents|InputAxisCannonsUpDown
  (params (AxisValue :type Float%20%28single-precision%29))
  (Default|RotateCannonsPitch (Variables|Default|GetArtilleryComponent) AxisValue))

(event Input|AxisEvents|InputAxisRotateShipRight
  (params (AxisValue :type Float%20%28single-precision%29))
  (Transformation|AddActorLocalRotation (Math|Rotator|MakeRotator 0.0 0.0 AxisValue) false false))

(event Input|AxisEvents|InputAxisAimCannonsAxis
  (params (AxisValue :type Float%20%28single-precision%29))
  (bind _artillerycomponent (Variables|Default|GetArtilleryComponent))
  (if (> AxisValue 0.0)
    (Variables|/Game/Blueprints/Components/ArtilleryComponent.ArtilleryComponent_C|SetIsAiming _artillerycomponent true)
    (Default|DrawTrajectory (Variables|Default|GetArtilleryComponent))
    (else
      (Variables|/Game/Blueprints/Components/ArtilleryComponent.ArtilleryComponent_C|SetIsAiming _artillerycomponent false))))

(fn ConstructionScript)