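; Ship artillery component that spawns and attaches a cannon at each CannonPlace on its owning pawn, then controls their pitch and firing.
; Shoot broadcasts OnShoot with the ball type, gated by a cooldown timer.
; While aiming, DrawTrajectory debug-draws a predicted path from a ship-centred muzzle point using the ball type's speed.
; Cannon selection is unfinished: it debug-draws the target/cursor direction but returns the first negative-yaw place.
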(event EventBeginPlay
  (bind _returnvalue (Components|GetOwner))
  (bind _aspawn (Utilities|Casting|CastToPawn _returnvalue))
  (Variables|Default|SetOwnerPawn _aspawn)
  (bind _asplayer_controller (Utilities|Casting|CastToPlayerController (Pawn|GetController _aspawn)))
  (Variables|Default|SetOwnerPlayerController _asplayer_controller)
  (bind _output_get (Variables|Default|SetCannonPlaces (Actor|GetComponentsByClass _returnvalue "/Game/Blueprints/Components/CannonPlaceComponent.CannonPlaceComponent_C")))
  (for _array_element _output_get
    (bind _outcannon (CallFunction|SetupCannon _array_element))
    (Variables|/Game/Blueprints/Components/CannonPlaceComponent.CannonPlaceComponent_C|SetCannon _array_element _outcannon)))

(event EventTick
  (params (DeltaSeconds :type Float%20%28single-precision%29)))

(fn SetupCannon
  (params (InCannonPlace :type Cannon%20Place%20Component%20Object%20Reference))
  (bind _ownerpawn (Variables|Default|GetOwnerPawn))
  (Utilities|IsValid _ownerpawn
    (:Is%20Valid
      (bind _returnvalue (Game|SpawnActorfromClass "/Game/Blueprints/Cannon.Cannon_C" (Transformation|GetWorldTransform InCannonPlace) "Undefined" _ownerpawn 0 self (Variables|Default|GetCannonsYawSpeed) _ownerpawn))
      (Transformation|AttachActorToActor _returnvalue (Variables|Default|GetOwnerPawn) "None" "KeepWorld" "KeepWorld" "KeepWorld" true)
      (return _returnvalue))))

(fn Shoot
  (if (Variables|Default|GetCanShoot)
    (Default|CallOnShoot (Variables|Default|GetBallType))
    (Variables|Default|SetCanShoot false)
    (Utilities|Time|SetTimerbyFunctionName 0 "Shoot Cooldown Ended" (Variables|Default|GetTimeBetweenShots))))

(fn ShootCooldownEnded
  (Variables|Default|SetCanShoot true))

(fn RotateCannonsPitch
  (params (Value :type Float%20%28single-precision%29))
  (for _array_element (Variables|Default|GetCannonPlaces)
    (Default|TrytoAddPitchRotation (Variables|/Game/Blueprints/Components/CannonPlaceComponent.CannonPlaceComponent_C|GetCannon _array_element) (* Value (Utilities|Time|GetWorldDeltaSeconds) (Variables|Default|GetCannonsPitchSpeed)))))

(fn DrawTrajectory
  (if (Variables|Default|GetIsAiming)
    (bind _outcannonplace (CallFunction|GetClosestCannonPlace))
    (LocalVariables|SetCannonPlace _outcannonplace)
    (CallFunction|PredictBallPath (LocalVariables|GetCannonPlace))))

(fn GetClosestCannonPlace
  (bind _ownerpawn (Variables|Default|GetOwnerPawn))
  (bind _returnvalue (Transformation|GetActorLocation _ownerpawn))
  (bind _targetdirection (CallFunction|GetShootDirection))
  (LocalVariables|SetTargetDirection _targetdirection)
  (Development|PrintString "Hello")
  (Rendering|Debug|DrawDebugLine _returnvalue (+ _returnvalue (* (Math|Rotator|GetRotationXVector (LocalVariables|GetTargetDirection)) 1e+03)) "(R=1.000000,G=0.000000,B=0.021455,A=1.000000)" 0.0 1e+01)
  (for _array_element (Variables|Default|GetCannonPlaces)
    (if (< (.yaw (Variables|/Script/Engine.SceneComponent|GetRelativeRotation _array_element)) 0.0)
      (return _array_element))))

(fn PredictBallPath
  (params (InCannonPlace :type Cannon%20Place%20Component%20Object%20Reference))
  (bind _ballconfig (Variables|Default|GetBallConfig))
  (bind _outmuzzlelocation (CallFunction|GetMiddleCannonMuzzle InCannonPlace))
  (bind _predictresult (Class|GameplayStatics|BlueprintPredictProjectilePathAdvanced (Utilities|Struct|MakePredictProjectilePathParams _outmuzzlelocation (* (Math|Vector|GetForwardVector (Transformation|GetWorldRotation (Variables|/Game/Blueprints/Cannon.Cannon_C|GetBallSpawnPoint (Variables|/Game/Blueprints/Components/CannonPlaceComponent.CannonPlaceComponent_C|GetCannon InCannonPlace)))) (Utilities|Select :Index (Variables|Default|GetBallType) :NewEnumerator0 (.roundshotspeed _ballconfig) :NewEnumerator1 (.buckshotspeed _ballconfig) :NewEnumerator2 (.knippelspeed _ballconfig))) true 0.0 5.0 true "ECC_WorldStatic" "ObjectTypeQuery1")))
  (for _array_element (.PathData (Utilities|Struct|BreakPredictProjectilePathResult _predictresult))
    (Rendering|Debug|DrawDebugSphere (.Location (Utilities|Struct|BreakPredictProjectilePathPointData _array_element)) 2e+01 12 "(R=1.000000,G=0.042986,B=0.000000,A=1.000000)" 0.0)))

(fn GetMiddleCannonMuzzle
  (params (InCannonPlace :type Cannon%20Place%20Component%20Object%20Reference))
  (bind _relativelocation (Variables|/Script/Engine.SceneComponent|GetRelativeLocation InCannonPlace))
  (bind _ownerpawn (Variables|Default|GetOwnerPawn))
  ;[1 1 1] Ищем позицию дула пушки в нуле по Х относительно пивота корабля
  (return (+ (- (Transformation|GetWorldLocation (Variables|/Game/Blueprints/Cannon.Cannon_C|GetBallSpawnPoint (Variables|/Game/Blueprints/Components/CannonPlaceComponent.CannonPlaceComponent_C|GetCannon InCannonPlace))) (Transformation|GetWorldLocation InCannonPlace)) (Math|Vector|RotateVector (Math|Vector|MakeVector 0.0 (.y _relativelocation) (.z _relativelocation)) (Transformation|GetActorRotation _ownerpawn)) (Transformation|GetActorLocation _ownerpawn))))

(fn GetShootDirection
  (Utilities|IsValid (Variables|Default|GetShootTarget)
    (:Is%20Valid
      (return (Math|Rotator|FindLookatRotation (Transformation|GetActorLocation (Variables|Default|GetOwnerPawn)) (Transformation|GetActorLocation (Variables|Default|GetShootTarget)))))
    (:Is%20Not%20Valid
      (return (Math|Rotator|FindLookatRotation (Transformation|GetActorLocation (Variables|Default|GetOwnerPawn)) (.Location (Collision|BreakHitResult (.HitResult (Game|Player|GetHitResultUnderCursorbyChannel (Variables|Default|GetOwnerPlayerController) "TraceTypeQuery1" true)))))))))