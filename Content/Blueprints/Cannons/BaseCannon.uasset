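; Base cannon actor that aims and fires for its owner's ArtilleryComponent.
; Each tick it turns base yaw and muzzle pitch toward the component's target at constant speed within CannonShootData limits, re-centering yaw when the target is over 90 degrees off.
; The component's OnShoot event spawns the given ball class and Niagara effect, only if yaw deviation is acceptable and the timer-based cooldown has ended.
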(event Custom|OnShoot_Event
  (params (CannonBall :type Cannon%20Ball%20Projectile%20Class%20Reference))
  (CallFunction|TrytoShootBall CannonBall))

(event EventBeginPlay
  (bind _artillerycomponent (Variables|Default|GetArtilleryComponent))
  (Utilities|IsValid _artillerycomponent
    (:Is%20Valid
      (EventDispatchers|BindEventtoOnShoot _artillerycomponent (delegate Custom|OnShoot_Event)))))

(event EventTick
  (params (DeltaSeconds :type Float%20%28single-precision%29))
  (bind _returnvalue (Components|GetOwner))
  (bind _returnvalue_2 (Actor|GetComponentbyClass _returnvalue "/Game/Blueprints/ArtillerySystem/Components/ArtilleryComponent.ArtilleryComponent_C"))
  (Utilities|IsValid _returnvalue
    (:Is%20Valid
      (CallFunction|SetCannonsYawRotation (Default|GetShootTargetLocation _returnvalue_2) DeltaSeconds)
      (CallFunction|SetCannonsPitchRotation (Default|GetShoottoTargetRotation _returnvalue_2) DeltaSeconds))))

(fn ConstructionScript)

(fn TrytoShootBall
  (params (BallType :type Cannon%20Ball%20Projectile%20Class%20Reference))
  (if (and (CallFunction|IsYawDeviationAcceptable (Variables|Default|GetLookAtTargetRotation)) (Variables|Default|GetCanShoot))
    (CallFunction|ShootBall BallType)))

(fn ShootBall
  (params (BallType :type Cannon%20Ball%20Projectile%20Class%20Reference))
  (bind _ballspawnpoint (Variables|Default|GetBallSpawnPoint))
  (bind _returnvalue (Transformation|GetWorldTransform _ballspawnpoint))
  (Game|SpawnActorfromClass BallType (Transformation|GetWorldTransform (Variables|Default|GetBallSpawnPoint)) "Undefined" (Components|GetOwner) (Game|GetInstigator))
  (Niagara|SpawnSystematLocation (Variables|Defaults|GetShootNiagaraSystem) (.location _returnvalue) (.rotation _returnvalue) (.scale _returnvalue))
  (Variables|Default|SetCanShoot false)
  (Utilities|Time|SetTimerbyFunctionName 0 "Shoot Cooldown Ended" (.TimeBetweenShots (Utilities|Struct|BreakCannonShootData (Variables|Defaults|GetCannonShootData)))))

(fn SetCannonsPitchRotation
  (params (TargetWorldRotation :type Rotator) (DeltaTIme :type Float%20%28single-precision%29))
  (bind _cannonshootdata (Variables|Defaults|GetCannonShootData))
  (bind _cannonmuzzlepivot (Variables|Default|GetCannonMuzzlePivot))
  (bind (_maxcannonyawangle _maxcannonpitchangle _defaultcannonpitchangle) (Utilities|Struct|BreakCannonShootData _cannonshootdata))
  (Transformation|SetRelativeRotation (Variables|Default|GetCannonMuzzlePivot) (Math|Rotator|MakeRotator 0.0 (Math|Interpolation|FInterptoConstant (.Pitch (Math|Rotator|BreakRotator (Variables|/Script/Engine.SceneComponent|GetRelativeRotation (Variables|Default|GetCannonMuzzlePivot)))) (Math|Float|ClampAngle (+ (.pitch (Math|Rotator|Delta(Rotator) TargetWorldRotation (Transformation|GetWorldRotation _cannonmuzzlepivot))) (.pitch (Variables|/Script/Engine.SceneComponent|GetRelativeRotation _cannonmuzzlepivot))) (- _defaultcannonpitchangle _maxcannonpitchangle) (+ _maxcannonpitchangle _defaultcannonpitchangle)) DeltaTIme (.PitchRotationSpeed (Utilities|Struct|BreakCannonShootData (Variables|Defaults|GetCannonShootData)))) 0.0) false false))

(fn SetCannonsYawRotation
  (params (TargetWorldLocation :type Vector) (DeltaTime :type Float%20%28single-precision%29))
  (bind _cannonbase (Variables|Default|GetCannonBase))
  (bind _cannonshootdata (Variables|Defaults|GetCannonShootData))
  (bind _maxcannonyawangle (Utilities|Struct|BreakCannonShootData _cannonshootdata))
  (bind _output_get (Variables|Default|SetLookAtTargetRotation (Math|Rotator|FindLookatRotation (Transformation|GetActorLocation) TargetWorldLocation)))
  ;[1 1 1] Можно соединить True и Set 0.0 чтобы пушки на противоположной стороне возвращались в 0 положение
  (if (> (Math|Float|Absolute(Float) (+ (.Yaw (Math|Rotator|BreakRotator (Math|Rotator|Delta(Rotator) _output_get (Transformation|GetWorldRotation _cannonbase)))) (.yaw (Variables|/Script/Engine.SceneComponent|GetRelativeRotation _cannonbase)))) 9e+01)
    (LocalVariables|SetFinalAngle 0.0)
    (else
      (LocalVariables|SetFinalAngle (Math|Float|ClampAngle (+ (.Yaw (Math|Rotator|BreakRotator (Math|Rotator|Delta(Rotator) _output_get (Transformation|GetWorldRotation _cannonbase)))) (.yaw (Variables|/Script/Engine.SceneComponent|GetRelativeRotation _cannonbase))) (* _maxcannonyawangle -1.0) _maxcannonyawangle))))
  (Transformation|SetRelativeRotation (Variables|Default|GetCannonBase) (Math|Rotator|MakeRotator 0.0 0.0 (Math|Interpolation|FInterptoConstant (.Yaw (Math|Rotator|BreakRotator (Variables|/Script/Engine.SceneComponent|GetRelativeRotation (Variables|Default|GetCannonBase)))) (LocalVariables|GetFinalAngle) DeltaTime (.YawRotationSpeed (Utilities|Struct|BreakCannonShootData (Variables|Defaults|GetCannonShootData))))) false false))

(fn IsYawDeviationAcceptable
  (params (ShootDirection :type Rotator))
  (bind _cannonshootdata (Variables|Defaults|GetCannonShootData))
  (bind (_maxcannonyawangle _maxcannonpitchangle _defaultcannonpitchangle _yawrotationspeed _pitchrotationspeed _cannonshootingdeviationangle) (Utilities|Struct|BreakCannonShootData _cannonshootdata))
  (return (<= (Math|Float|Absolute(Float) (.yaw (Math|Rotator|Delta(Rotator) ShootDirection (Transformation|GetActorRotation)))) (+ _maxcannonyawangle _cannonshootingdeviationangle))))

(fn ShootCooldownEnded
  (Variables|Default|SetCanShoot true))

(fn SetCannonShootData
  (params (CannonShootData :type Cannon%20Shoot%20Data%20Structure))
  (Variables|Defaults|SetCannonShootData CannonShootData))