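; Cannon actor that aims at its owner pawn's artillery target and fires projectiles with a Niagara effect.
; Each tick it turns base yaw and muzzle pitch at constant speed within angle limits, recentring yaw for targets over 90 degrees off.
; The ArtilleryComponent's OnShoot event spawns the given projectile only if yaw deviation from the actor's facing is acceptable.
; The pitch deviation check is defined but unused.
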(event Custom|OnShoot_Event
  (params (ProjectileClass :type Cannon%20Ball%20Projectile%20Class%20Reference) (ShootDirection :type Rotator))
  (CallFunction|TrytoShootBall ProjectileClass ShootDirection))

(event EventBeginPlay
  (bind _artillerycomponent (Variables|Default|GetArtilleryComponent))
  (Utilities|IsValid _artillerycomponent
    (:Is%20Valid
      (EventDispatchers|BindEventtoOnShoot _artillerycomponent (delegate Custom|OnShoot_Event)))))

(event EventTick
  (params (DeltaSeconds :type Float%20%28single-precision%29))
  (bind _ownerpawn (Variables|Default|GetOwnerPawn))
  (bind _returnvalue (Actor|GetComponentbyClass _ownerpawn "/Game/Blueprints/Components/ArtilleryComponent.ArtilleryComponent_C"))
  (Utilities|IsValid _ownerpawn
    (:Is%20Valid
      (CallFunction|SetCannonsYawRotation (Variables|/Game/Blueprints/Components/ArtilleryComponent.ArtilleryComponent_C|GetLookAtTargetRotation _returnvalue) DeltaSeconds)
      (CallFunction|SetCannonsPitchRotation (Math|Conversions|RotationFromXVector (Variables|/Game/Blueprints/Components/ArtilleryComponent.ArtilleryComponent_C|GetShootToTargetDirection _returnvalue)) DeltaSeconds))))

(fn ConstructionScript
  (Variables|Default|SetDefaultPitchRotation (.Pitch (Math|Rotator|BreakRotator (Variables|/Script/Engine.SceneComponent|GetRelativeRotation (Variables|Default|GetCannonMuzzlePivot))))))

(fn TrytoShootBall
  (params (BallType :type Cannon%20Ball%20Projectile%20Class%20Reference) (ShootDirection :type Rotator))
  (if (CallFunction|IsYawDeviationAcceptable ShootDirection)
    (CallFunction|ShootBall BallType)))

(fn ShootBall
  (params (BallType :type Cannon%20Ball%20Projectile%20Class%20Reference))
  (bind _ballspawnpoint (Variables|Default|GetBallSpawnPoint))
  (bind _returnvalue (Transformation|GetWorldTransform _ballspawnpoint))
  (Game|SpawnActorfromClass BallType (Transformation|GetWorldTransform (Variables|Default|GetBallSpawnPoint)) "Undefined" (Components|GetOwner) (Game|GetInstigator))
  (Niagara|SpawnSystematLocation (Variables|Defaults|GetShootNiagaraSystem) (.location _returnvalue) (.rotation _returnvalue) (.scale _returnvalue)))

(fn GetRelativeRotations
  (bind _returnvalue (Transformation|GetActorRotation))
  (bind _ownerpawn (Variables|Default|GetOwnerPawn))
  (bind _returnvalue_2 (Transformation|GetActorRotation _ownerpawn))
  (bind _returnvalue_3 (Math|Rotator|Delta(Rotator) _returnvalue_2 _returnvalue))
  (Utilities|IsValid _ownerpawn
    (:Is%20Valid
      (return (.pitch _returnvalue_3) (.yaw _returnvalue_3)))))

(fn SetCannonsPitchRotation
  (params (TargetWorldRotation :type Rotator) (DeltaTIme :type Float%20%28single-precision%29))
  (bind _cannonmuzzlepivot (Variables|Default|GetCannonMuzzlePivot))
  (Transformation|SetRelativeRotation (Variables|Default|GetCannonMuzzlePivot) (Math|Rotator|MakeRotator 0.0 (Math|Interpolation|FInterptoConstant (.Pitch (Math|Rotator|BreakRotator (Variables|/Script/Engine.SceneComponent|GetRelativeRotation (Variables|Default|GetCannonMuzzlePivot)))) (Math|Float|ClampAngle (+ (.pitch (Math|Rotator|Delta(Rotator) TargetWorldRotation (Transformation|GetWorldRotation _cannonmuzzlepivot))) (.pitch (Variables|/Script/Engine.SceneComponent|GetRelativeRotation _cannonmuzzlepivot))) (- (Variables|Default|GetDefaultPitchRotation) (Variables|Defaults|GetMaxPitchAngle)) (+ (Variables|Default|GetDefaultPitchRotation) (Variables|Defaults|GetMaxPitchAngle))) DeltaTIme (Variables|Defaults|GetPitchRotationSpeed)) 0.0) false false))

(fn SetCannonsYawRotation
  (params (TargetWorldRotation :type Rotator) (DeltaTime :type Float%20%28single-precision%29))
  (bind _cannonbase (Variables|Default|GetCannonBase))
  (bind _maxyawangle (Variables|Defaults|GetMaxYawAngle))
  (bind _returnvalue (Transformation|GetWorldRotation _cannonbase))
  (bind _relativerotation (Variables|/Script/Engine.SceneComponent|GetRelativeRotation _cannonbase))
  (bind _returnvalue_2 (Math|Rotator|Delta(Rotator) TargetWorldRotation _returnvalue))
  (bind _yaw (Math|Rotator|BreakRotator _returnvalue_2))
  (bind _returnvalue_3 (+ _yaw (.yaw _relativerotation)))
  ;[1 1 1] Можно соединить True и Set 0.0 чтобы пушки на противоположной стороне возвращались в 0 положение
  (if (> (Math|Float|Absolute(Float) _returnvalue_3) 9e+01)
    (LocalVariables|SetFinalAngle 0.0)
    (else
      (LocalVariables|SetFinalAngle (Math|Float|ClampAngle _returnvalue_3 (* _maxyawangle -1.0) _maxyawangle))))
  (Transformation|SetRelativeRotation (Variables|Default|GetCannonBase) (Math|Rotator|MakeRotator 0.0 0.0 (Math|Interpolation|FInterptoConstant (.Yaw (Math|Rotator|BreakRotator (Variables|/Script/Engine.SceneComponent|GetRelativeRotation (Variables|Default|GetCannonBase)))) (LocalVariables|GetFinalAngle) DeltaTime (Variables|Defaults|GetYawRotationSpeed))) false false))

(fn IsYawDeviationAcceptable
  (params (ShootDirection :type Rotator))
  (return (<= (Math|Float|Absolute(Float) (.yaw (Math|Rotator|Delta(Rotator) ShootDirection (Transformation|GetActorRotation)))) (+ (Variables|Default|GetMaxShootingAngle) (Variables|Defaults|GetMaxYawAngle)))))

(fn IsPitchDeviationAcceptable
  (params (ShootDirection :type Rotator))
  (return (<= (Math|Float|Absolute(Float) (.pitch (Math|Rotator|Delta(Rotator) ShootDirection (Transformation|GetWorldRotation (Variables|Default|GetCannonMuzzlePivot))))) (Variables|Default|GetMaxShootingAngle))))