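; Buckshot variant of a cannon projectile that randomizes its damage each time it spawns.
; On BeginPlay, after running the parent logic, it rewrites BallConfig, setting a fixed first field and scaling Damage by a random integer between the minimum and maximum damage multipliers.
; All other behavior comes from the parent class; Tick and overlap events are disabled.
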(event EventBeginPlay
  (|CallParentFunction)
  (Variables|Default|SetBallConfig (Utilities|Struct|MakeCannonBallConfig 1e+03 (* (Math|Random|RandomIntegerinRange (Variables|Default|GetMinDamageMultiplier) (Variables|Default|GetMaxDamageMultiplier)) (.damage (Variables|Default|GetBallConfig))) 0 0)))

(event Collision|EventActorBeginOverlap
  (params (OtherActor :type Actor%20Object%20Reference))
  (|CallParentFunction OtherActor) ; This node is disabled and will not be called.\nDrag off pins to build functionality.
)

(event EventTick
  (params (DeltaSeconds :type Float%20%28single-precision%29))
  (|CallParentFunction DeltaSeconds) ; This node is disabled and will not be called.\nDrag off pins to build functionality.
)

(fn ConstructionScript
  (|CallParentFunction))