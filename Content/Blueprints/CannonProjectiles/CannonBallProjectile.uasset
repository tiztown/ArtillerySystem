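; Cannonball projectile whose speed, mesh, damage and explosion effect all come from its BallConfig.
; The construction script applies the configured mesh to BallMesh and sets both initial and max speed on ProjectileMovement.
; On hit, it damages the other actor using the instigator's controller and the instigator as damage causer, spawns the explosion effect at its own transform, then destroys itself.
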(event EventBeginPlay)

(event Collision|EventActorBeginOverlap
  (params (OtherActor :type Actor%20Object%20Reference)))

(event EventTick
  (params (DeltaSeconds :type Float%20%28single-precision%29)))

(event Collision|EventHit
  (params (MyComp :type Primitive%20Component%20Object%20Reference) (Other :type Actor%20Object%20Reference) (OtherComp :type Primitive%20Component%20Object%20Reference) (bSelfMoved :type Boolean) (HitLocation :type Vector :default "0, 0, 0") (HitNormal :type Vector :default "0, 0, 0") (NormalImpulse :type Vector :default "0, 0, 0") (Hit :type Hit%20Result%20Structure%20%28by%20ref%29))
  (bind _returnvalue (Transformation|GetActorTransform))
  (bind _returnvalue_2 (Game|GetInstigator))
  (bind _ballconfig (Variables|Default|GetBallConfig))
  (bind (_speed _damage _staticmesh _explodeeffect) (Utilities|Struct|BreakCannonBallConfig _ballconfig))
  (Game|Damage|ApplyDamage Other _damage (Pawn|GetController _returnvalue_2) _returnvalue_2)
  (Niagara|SpawnSystematLocation _explodeeffect (.location _returnvalue) (.rotation _returnvalue) (.scale _returnvalue))
  (Actor|DestroyActor))

(fn ConstructionScript
  (bind _projectilemovement (Variables|Default|GetProjectileMovement))
  (bind _ballconfig (Variables|Default|GetBallConfig))
  (bind (_speed _damage _staticmesh) (Utilities|Struct|BreakCannonBallConfig _ballconfig))
  (Variables|/Script/Engine.ProjectileMovementComponent|SetMaxSpeed _projectilemovement _speed)
  (Variables|/Script/Engine.ProjectileMovementComponent|SetInitialSpeed _projectilemovement _speed)
  (Components|StaticMesh|SetStaticMesh (Variables|Default|GetBallMesh) _staticmesh))