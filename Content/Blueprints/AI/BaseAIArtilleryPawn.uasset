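; Base pawn Blueprint for AI artillery that targets the player through an ArtilleryComponent.
; Ten seconds after BeginPlay, it sets the first player controller's pawn as the component's shoot target, with no later retargeting.
; Tick prints the current target's name on screen every frame as debug output.
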(event EventBeginPlay
  (|CallParentFunction)
  (Utilities|FlowControl|Delay 1e+01)
  (Default|SetShootTarget (Variables|Default|GetArtilleryComponent) (Pawn|GetControlledPawn (Game|GetPlayerController 0))))

(event Collision|EventActorBeginOverlap
  (params (OtherActor :type Actor%20Object%20Reference))
  (|CallParentFunction OtherActor) ; This node is disabled and will not be called.\nDrag off pins to build functionality.
)

(event EventTick
  (params (DeltaSeconds :type Float%20%28single-precision%29))
  (|CallParentFunction DeltaSeconds)
  (Development|PrintString (Utilities|String|Append "Target is :" (Utilities|GetDisplayName (Default|GetShootTarget (Variables|Default|GetArtilleryComponent)))) true true "(R=0.000000,G=0.660000,B=1.000000,A=1.000000)" 0.0))

(fn ConstructionScript
  (|CallParentFunction))